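; BP_Microwave is an interactable microwave that collects ingredients carried by the first-person player.
; On BeginPlay it caches the game mode, its ingredient count and the player character.
; Interact moves the character's current ingredient into IngredientList, clears the held state and prints every stored name, or prints "non" when empty-handed.
; The cached count is not used afterwards, and no cooking logic is present.
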(event EventBeginPlay
  (bind _asbp_first_person_game_mode (Utilities|Casting|CastToBP_FirstPersonGameMode (Game|GetGameMode)))
  (bind _output_get (Variables|Default|SetGameModeRef _asbp_first_person_game_mode))
  (Variables|Default|SetNbIngredients (Variables|/Game/FirstPerson/Blueprints/BP_FirstPersonGameMode.BP_FirstPersonGameMode_C|GetNb%20Ingredients _output_get))
  (bind _asbp_first_person_character (Utilities|Casting|CastToBP_FirstPersonCharacter (Game|GetPlayerCharacter 0)))
  (Variables|Default|SetCharacterRef _asbp_first_person_character))

(event EventInteract
  (bind _characterref (Variables|Default|GetCharacterRef))
  (if (Variables|/Game/FirstPerson/Blueprints/BP_FirstPersonCharacter.BP_FirstPersonCharacter_C|GetbHasIngredient (Variables|Default|GetCharacterRef))
    (Utilities|Array|Add (Variables|Default|GetIngredientList) (Variables|/Game/FirstPerson/Blueprints/BP_FirstPersonCharacter.BP_FirstPersonCharacter_C|GetCurrentIngredient _characterref))
    (Variables|/Game/FirstPerson/Blueprints/BP_FirstPersonCharacter.BP_FirstPersonCharacter_C|SetCurrentIngredient _characterref 0)
    (Variables|/Game/FirstPerson/Blueprints/BP_FirstPersonCharacter.BP_FirstPersonCharacter_C|SetbHasIngredient _characterref false)
    (for _array_element (Variables|Default|GetIngredientList)
      (Development|PrintString (Variables|/Game/BP_Ingredient.BP_Ingredient_C|GetName _array_element)))
    (else
      (Development|PrintString "non"))))

(fn ConstructionScript)