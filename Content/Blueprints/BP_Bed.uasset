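; BP_Bed is an interactable bed that ends the day in the first-person game.
; It caches the BP_FirstPersonGameMode on BeginPlay and, on Interact, only allows sleep once the ingredient count reaches zero.
; Sleeping triggers the game mode's day summary and, if a hallucination item was eaten that day, clears that flag and raises the hallucination level; otherwise it prints a debug refusal.
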(event EventInteract
  (bind _gamemoderef (Variables|Default|GetGameModeRef))
  (if (<= (Variables|/Game/FirstPerson/Blueprints/BP_FirstPersonGameMode.BP_FirstPersonGameMode_C|GetNb%20Ingredients (Variables|Default|GetGameModeRef)) 0)
    (Default|DaySummary (Variables|Default|GetGameModeRef))
    (if (Variables|/Game/FirstPerson/Blueprints/BP_FirstPersonGameMode.BP_FirstPersonGameMode_C|GetbHasEatenHallucinationToday _gamemoderef)
      (Variables|/Game/FirstPerson/Blueprints/BP_FirstPersonGameMode.BP_FirstPersonGameMode_C|SetbHasEatenHallucinationToday _gamemoderef false)
      (Math|Integer|IncrementInt (Variables|/Game/FirstPerson/Blueprints/BP_FirstPersonGameMode.BP_FirstPersonGameMode_C|GetHallucinationLevel _gamemoderef)))
    (else
      (Development|PrintString "pas dodo"))))

(event EventBeginPlay
  (bind _asbp_first_person_game_mode (Utilities|Casting|CastToBP_FirstPersonGameMode (Game|GetGameMode)))
  (Variables|Default|SetGameModeRef _asbp_first_person_game_mode))

(fn ConstructionScript)