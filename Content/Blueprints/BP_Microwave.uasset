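; BP_Microwave is an interactable microwave that takes the player's held ingredient and updates madness counters.
; On Interact it stores the ingredient, decrements the game mode's ingredient count, flags eaten hallucinations and calls the character's InMicrowave.
; It then rescans the whole list, matching hard-coded French names to increment per-day madness levels, so earlier ingredients count again each time.
; Only day three checks the current day; other days share the day-one and day-two checks.
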(event EventBeginPlay
  (bind _asbp_first_person_game_mode (Utilities|Casting|CastToBP_FirstPersonGameMode (Game|GetGameMode)))
  (Variables|Default|SetGameModeRef _asbp_first_person_game_mode)
  (bind _asbp_first_person_character (Utilities|Casting|CastToBP_FirstPersonCharacter (Game|GetPlayerCharacter 0)))
  (Variables|Default|SetCharacterRef _asbp_first_person_character))

(event EventTick
  (params (DeltaSeconds :type Float%20%28single-precision%29)))

(event EventInteract
  (bind _characterref (Variables|Default|GetCharacterRef))
  (bind _currentingredient (Variables|/Game/FirstPerson/Blueprints/BP_FirstPersonCharacter.BP_FirstPersonCharacter_C|GetCurrentIngredient _characterref))
  (if (Variables|/Game/FirstPerson/Blueprints/BP_FirstPersonCharacter.BP_FirstPersonCharacter_C|GetbHasIngredient (Variables|Default|GetCharacterRef))
    (Utilities|Array|Add (Variables|Default|GetIngredientList) _currentingredient)
    (Math|Integer|DecrementInt (Variables|/Game/FirstPerson/Blueprints/BP_FirstPersonGameMode.BP_FirstPersonGameMode_C|GetNb%20Ingredients (Variables|Default|GetGameModeRef))
      (:%20%20
        (if (not (Variables|/Game/Blueprints/BP_Ingredient.BP_Ingredient_C|GetbNormal _currentingredient))
          (Variables|/Game/FirstPerson/Blueprints/BP_FirstPersonGameMode.BP_FirstPersonGameMode_C|SetbHasEatenHallucinationToday (Variables|Default|GetGameModeRef) true))
        (Default|InMicrowave _characterref)
        (for _array_element (Variables|Default|GetIngredientList)
          (if (== (Variables|/Game/FirstPerson/Blueprints/BP_FirstPersonGameMode.BP_FirstPersonGameMode_C|GetNbDay (Variables|Default|GetGameModeRef)) 3)
            (if (Math|Boolean|ORBoolean (Utilities|Enum|Equal(Enum) (Variables|/Game/Blueprints/BP_Ingredient.BP_Ingredient_C|GetName _array_element) "Pomme") (Utilities|Enum|Equal(Enum) (Variables|/Game/Blueprints/BP_Ingredient.BP_Ingredient_C|GetName _array_element) "Moutarde") (Utilities|Enum|Equal(Enum) (Variables|/Game/Blueprints/BP_Ingredient.BP_Ingredient_C|GetName _array_element) "Pain"))
              (Math|Integer|IncrementInt (Variables|Default|GetMadnessLevelDay3)))
            (elif (or (Utilities|Enum|Equal(Enum) (Variables|/Game/Blueprints/BP_Ingredient.BP_Ingredient_C|GetName _array_element) "Riz") (Utilities|Enum|Equal(Enum) (Variables|/Game/Blueprints/BP_Ingredient.BP_Ingredient_C|GetName _array_element) "Pâtes"))
              (Math|Integer|IncrementInt (Variables|Default|GetMadnessLevelDay1))
              (elif (or (Utilities|Enum|Equal(Enum) (Variables|/Game/Blueprints/BP_Ingredient.BP_Ingredient_C|GetName _array_element) "Yaourt nature") (Utilities|Enum|Equal(Enum) (Variables|/Game/Blueprints/BP_Ingredient.BP_Ingredient_C|GetName _array_element) "Sel"))
                (Math|Integer|IncrementInt (Variables|Default|GetMadnessLevelDay2))))))))))

(fn ConstructionScript)