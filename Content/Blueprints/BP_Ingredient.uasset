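; BP_Ingredient is an ingredient actor that the first-person player can pick up.
; On BeginPlay it maps its ingredient enum to a DT_Ingredients row, which supplies the mesh, name and Normal value.
; Interact calls Grab when it is not already held and the character has no ingredient.
; Grab flags it as held, disables mesh collision and attaches it to the character's Scene component, keeping world rotation.
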(event EventBeginPlay
  (bind _asbp_first_person_character (Utilities|Casting|CastToBP_FirstPersonCharacter (Game|GetPlayerCharacter 0)))
  (Variables|Default|SetCharacterRef _asbp_first_person_character)
  (bind _returnvalue (Utilities|GetDataTableRow "/Game/DataTables/DT_Ingredients.DT_Ingredients" (Utilities|Select :Index (Variables|Default|GetEnumIngredient) :NewEnumerator0 "Mustard" :NewEnumerator1 "Pasta" :NewEnumerator2 "Rice" :NewEnumerator3 "GroundBeef" :NewEnumerator4 "Bread" :NewEnumerator5 "Apple" :NewEnumerator6 "Salt" :NewEnumerator7 "HotWater" :NewEnumerator8 "InstantNoodles" :NewEnumerator9 "BreadedFish" :NewEnumerator10 "BellPepper" :NewEnumerator11 "PlainYogurt" :NewEnumerator12 "Moss" :NewEnumerator13 "StrangeShroom" :NewEnumerator14 "ToiletWater" :NewEnumerator15 "BlackMold" :NewEnumerator16 "DeadRat" :NewEnumerator17 "Shampoo"))
    (:then
      (Components|StaticMesh|SetStaticMesh (Variables|Default|GetMesh) (.mesh (Utilities|Struct|BreakS_Ingredient _returnvalue)))
      (Variables|Default|SetName (Utilities|String|EnumtoString (.name (Utilities|Struct|BreakS_Ingredient _returnvalue))))
      (Variables|Default|SetbNormal (.normal (Utilities|Struct|BreakS_Ingredient _returnvalue))))))

(event EventInteract
  (if (and (not (Variables|Default|GetbIsGrabbed)) (not (Variables|/Game/FirstPerson/Blueprints/BP_FirstPersonCharacter.BP_FirstPersonCharacter_C|GetbHasIngredient (Variables|Default|GetCharacterRef))))
    (CallFunction|Grab)))

(fn ConstructionScript)

(fn Grab
  (Variables|Default|SetbIsGrabbed true)
  (Collision|SetCollisionEnabled (Variables|Default|GetMesh) "NoCollision")
  (Transformation|AttachComponentToComponent (Variables|/Game/FirstPerson/Blueprints/BP_FirstPersonCharacter.BP_FirstPersonCharacter_C|GetScene (Variables|Default|GetCharacterRef)) "None" "SnapToTarget" "KeepWorld" "KeepRelative" false))