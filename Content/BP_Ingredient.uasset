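; BP_Ingredient is a pickup ingredient actor that the first-person player can grab.
; On BeginPlay it applies its configured mesh and caches the player character reference.
; Interact calls Grab once, which disables mesh collision and attaches it to the character's Scene component, snapping location while keeping world rotation.
; An unused Select over an ingredient enum remains in the graph, and no drop logic exists.
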(event EventBeginPlay
  (Components|StaticMesh|SetStaticMesh (Variables|Default|GetMesh) (Variables|Default|GetIngredientMesh))
  (bind _asbp_first_person_character (Utilities|Casting|CastToBP_FirstPersonCharacter (Game|GetPlayerCharacter 0)))
  (Variables|Default|SetCharacterRef _asbp_first_person_character))

(event EventInteract
  (if (not (Variables|Default|GetbIsGrabbed))
    (CallFunction|Grab)
    (Development|PrintString (Utilities|String|ToString(Boolean) (Variables|Default|GetbIsGrabbed)))))

(fn ConstructionScript)

(fn Grab
  (Variables|Default|SetbIsGrabbed true)
  (Collision|SetCollisionEnabled (Variables|Default|GetMesh) "NoCollision")
  (Transformation|AttachComponentToComponent (Variables|/Game/FirstPerson/Blueprints/BP_FirstPersonCharacter.BP_FirstPersonCharacter_C|GetScene (Variables|Default|GetCharacterRef)) "None" "SnapToTarget" "KeepWorld" "KeepRelative" false))